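; Enemy Blueprint for an MMORPG that shows a floating health bar and name through its HpBar widget component.
; BeginPlay caches the HPBarEnenmy widget, and every Tick pushes normalized CurrentHP and NPCName into it.
; Tick also billboards the bar by rotating it toward the player character's follow camera.
; The graph holds only this display logic, with no AI, damage or death handling.
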(event EventBeginPlay
  ;[1 1 1] Get widget reference
  (Variables|Default|SetHPBarWidgetRef (.AsHPBar%20Enenmy (Utilities|Casting|CastToHPBarEnenmy (UserInterface|GetUserWidgetObject (Variables|Default|Get_hp_Bar))))))

(event Collision|EventActorBeginOverlap
  (params (OtherActor :type Actor%20Object%20Reference)))

(event EventTick
  (params (DeltaSeconds :type Float%20%28single-precision%29))
  ;[1 1 1] Auto widget rotation to camera
  (Utilities|FlowControl|Sequence
    (:then_0
      ;[1 1 1] Draw hp to widget
      (Progress|SetPercent (Variables|/Game/MMORPG/Enemy/HPBarEnenmy.HPBarEnenmy_C|Get_pb_HPBar (Variables|Default|GetHPBarWidgetRef)) (Math|Float|NormalizetoRange (Variables|Default|GetCurrentHP) 0.0 (Variables|Default|GetMaxHP)))
      ;[1 1 1] Draw name to widget
      (Rendering|Components|TextRender|SetText (Variables|/Game/MMORPG/Enemy/HPBarEnenmy.HPBarEnenmy_C|Get_tb_mobname (Variables|Default|GetHPBarWidgetRef)) (Variables|Default|GetNPCName)))
    (:then_1
      (Transformation|SetWorldRotation (Variables|Default|Get_hp_Bar) (Math|Rotator|FindLookatRotation (Transformation|GetWorldLocation (Variables|Default|Get_hp_Bar)) (Transformation|GetWorldLocation (Variables|/Game/MMORPG/PlayerController/BP_ThirdPersonCharacter.BP_ThirdPersonCharacter_C|GetFollowCamera (.AsBP%20Third%20Person%20Character (Utilities|Casting|CastToBP_ThirdPersonCharacter (Game|GetPlayerCharacter 0)))))) false false))))

(fn ConstructionScript)