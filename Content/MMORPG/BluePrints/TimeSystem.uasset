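; Time system actor that drives the day/night cycle and counts game days.
; The SunMovement timeline starts at StartTime with its play rate set by DaySpeed, and each Tick applies its tracks to sun rotation and directional and sky light intensity.
; The timeline's seconds track and Day form the Time timespan, with flags for hours 23 and 0 detecting midnight rollover to increment Day.
; A DisplayTime debug print exists but is never called.
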(event EventBeginPlay
  (bind (_direction _y _z _seconds _skylight _dirlight) (Timeline|Sun%20Movement SetNewTime)))

(event EventTick
  (params (DeltaSeconds :type Float%20%28single-precision%29))
  (CallFunction|TimeSystem)
  (Variables|Default|SetMovementSec (stale EventBeginPlay _seconds))
  (Transformation|SetActorRotation (Variables|Default|GetDirLight) (Math|Rotator|MakeRotator 0.0 (stale EventBeginPlay _y) (stale EventBeginPlay _z)))
  (Rendering|Components|Light|SetIntensity (Variables|/Script/Engine.SkyLight|GetLightComponent (Variables|Default|GetSkyLight)) (stale EventBeginPlay _skylight))
  (Rendering|Components|Light|SetIntensity (Variables|/Script/Engine.Light|GetLightComponent (Variables|Default|GetDirLight)) (stale EventBeginPlay _dirlight)))

(fn ConstructionScript
  (Components|Timeline|SetPlayRate (Variables|Default|GetSun%20Movement) (Variables|Default|GetDaySpeed)))

(fn TimeSystem
  (CallFunction|DayTickSystem)
  (Variables|Default|SetTime (Math|Timespan|MakeTimespan (Variables|Default|GetDay) 0 0 (Math|Float|Truncate (Variables|Default|GetMovementSec)))))

(fn DayTickSystem
  (bind _time (Variables|Default|GetTime))
  (Utilities|FlowControl|Sequence
    (:then_0
      (if (== (.hours (Variables|Default|GetTime)) 23)
        (Variables|Default|Set23 true)))
    (:then_1
      (if (== (.hours (Variables|Default|GetTime)) 0)
        (Variables|Default|Set00 true)))
    (:then_2
      (if (and (Variables|Default|Get23) (Variables|Default|Get00))
        (Variables|Default|SetDay (+ (Variables|Default|GetDay) 1))
        (Variables|Default|Set00 false)
        (Variables|Default|Set23 false)))
    (:then_3
      (if (and (>= (.hours _time) 23) (>= (.hours _time) 1))
        (Variables|Default|Set00 false)))))

(fn DisplayTime
  (bind _time (Variables|Default|GetTime))
  (Development|PrintString (Utilities|String|ToString(Text) (Utilities|Text|FormatText "Day: {Day}  {HH}:{mm}:{ss}" (Utilities|Text|ToText(Integer) (.days _time)) (Utilities|Text|ToText(Integer) (.hours _time)) (Utilities|Text|ToText(Integer) (.minutes _time)) (Utilities|Text|ToText(Integer) (.seconds _time)))) true true "(R=0.000000,G=0.660000,B=1.000000,A=1.000000)" 0.0))